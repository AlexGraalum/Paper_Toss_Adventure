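; Trash bin goal for a VR paper-ball throwing game that displays its score weight and reports scored throws.
; Every tick, the weight text turns toward the VRPawn camera, subtracting the bin's yaw from the look-at rotation.
; When the Paperstack's current ball overlaps GoalCollision, the bin destroys it, clears the stack's PaperPresent flag and calls the goal event with its ScoreWeight.
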(event OnComponentBeginOverlap(GoalCollision)
  (params (OverlappedComponent :type Primitive%20Component%20Object%20Reference) (OtherActor :type Actor%20Object%20Reference) (OtherComp :type Primitive%20Component%20Object%20Reference) (OtherBodyIndex :type Integer) (bFromSweep :type Boolean) (SweepResult :type Hit%20Result%20Structure%20%28by%20ref%29))
  ;[1 1 1] On Goal From Paperball Trigger
  (bind _returnvalue (Actor|GetActorOfClass "/Game/Blueprints/Paperstack.Paperstack_C"))
  (if (== (Variables|/Game/Blueprints/Paperstack.Paperstack_C|GetCurrentBall _returnvalue) OtherActor)
    (Actor|DestroyActor (Variables|/Game/Blueprints/Paperstack.Paperstack_C|GetCurrentBall _returnvalue))
    (bind _returnvalue_2 (Actor|GetActorOfClass "/Game/Blueprints/Paperstack.Paperstack_C"))
    (Variables|/Game/Blueprints/Paperstack.Paperstack_C|SetPaperPresent _returnvalue_2 false)
    (Default|CallGoalEvent (Variables|Default|GetScoreWeight))))

(event EventBeginPlay
  ;[1 1 1] Initialize Trashbin ScoreWeight Text Render
  (Rendering|Components|TextRender|SetText (Variables|Default|GetWeightText) (Utilities|Text|ToText(Integer) (Variables|Default|GetScoreWeight))))

(event EventTick
  (params (DeltaSeconds :type Float%20%28single-precision%29))
  (bind _weighttext (Variables|Default|GetWeightText))
  ;[1 1 1] Allign Trashbin ScoreWeight Text to VRPawn Camera
  (bind _returnvalue (Actor|GetActorOfClass "/Game/Blueprints/VRPawn.VRPawn_C"))
  (Transformation|SetRelativeRotation _weighttext (Math|Rotator|MakeRotator 0.0 (.Pitch (Math|Rotator|BreakRotator (Math|Rotator|FindLookatRotation (Transformation|GetWorldLocation _weighttext) (Transformation|GetWorldLocation (Variables|/Game/Blueprints/VRPawn.VRPawn_C|GetCamera _returnvalue))))) (- (.Yaw (Math|Rotator|BreakRotator (Math|Rotator|FindLookatRotation (Transformation|GetWorldLocation _weighttext) (Transformation|GetWorldLocation (Variables|/Game/Blueprints/VRPawn.VRPawn_C|GetCamera _returnvalue))))) (.Yaw (Math|Rotator|BreakRotator (Transformation|GetActorRotation))))) false false))

(fn ConstructionScript)