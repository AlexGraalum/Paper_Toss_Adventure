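; Chair obstacle actor that starts moving and rotating when the score passed to TriggerObstacle equals its TriggerScore.
; Start transform is cached on BeginPlay.
; While Activated, Tick plays two looping timelines that lerp location (with sweep) toward EndLocation and rotation toward EndRotation.
; Nothing stops the timelines, so clearing Activated does not halt motion already running.
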(event EventBeginPlay
  ;[1 1 1] Set Initial Location and Rotation
  (bind _output_get (Variables|Default|SetStartLocation (Transformation|GetActorLocation)))
  (bind _output_get_2 (Variables|Default|SetStartRotation (Transformation|GetActorRotation))))

(event Collision|EventActorBeginOverlap
  (params (OtherActor :type Actor%20Object%20Reference)))

(event EventTick
  (params (DeltaSeconds :type Float%20%28single-precision%29))
  (if (Variables|Default|GetActivated)
    (Utilities|FlowControl|Sequence
      (:then_0
        ;[1 1 1] Movement Timeline
        (bind (_direction _chair_move_track) (Timeline|Movement%20Timeline Play)
          (:Update
            ;[1 1 1] Location Lerp
            (Transformation|SetActorLocation (Math|Vector|Lerp(Vector) (stale EventBeginPlay _output_get) (Variables|Default|GetEndLocation) _chair_move_track) true false))
          (:Finished
            (switch Utilities|FlowControl|Switch|SwitchonETimelineDirection _direction
              (:Forward
                (Timeline|Movement%20Timeline PlayFromStart))
              (:Backward
                (Timeline|Movement%20Timeline ReverseFromEnd))))))
      (:then_1
        ;[1 1 1] Rotation Timeline
        (bind (_direction_2 _chair_move_track_2) (Timeline|Rotation%20Timeline Play)
          (:Update
            ;[1 1 1] Rotation Lerp
            (Transformation|SetActorRotation (Math|Rotator|Lerp(Rotator) (stale EventBeginPlay _output_get_2) (Variables|Default|GetEndRotation) _chair_move_track_2)))
          (:Finished
            (switch Utilities|FlowControl|Switch|SwitchonETimelineDirection _direction_2
              (:Forward
                (Timeline|Rotation%20Timeline PlayFromStart))
              (:Backward
                (Timeline|Rotation%20Timeline ReverseFromEnd)))))))))

(fn ConstructionScript)

(fn TriggerObstacle
  (params (Score :type Integer))
  (Variables|Default|SetActivated (== Score (Variables|Default|GetTriggerScore))))