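; Shop display actor where the player buys and selects paper ball variants by overlapping trigger components.
; Each trigger fires a selection event with an index, ball type and price, handled by TriggerSelection.
; An affordable unowned ball is marked purchased and the remaining money is sent through a purchase event.
; Overlapping an owned, unselected ball changes the Paperstack's ball and moves the "Selected" label.
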(event OnComponentBeginOverlap(PinkTrigger)
  (params (OverlappedComponent :type Primitive%20Component%20Object%20Reference) (OtherActor :type Actor%20Object%20Reference) (OtherComp :type Primitive%20Component%20Object%20Reference) (OtherBodyIndex :type Integer) (bFromSweep :type Boolean) (SweepResult :type Hit%20Result%20Structure%20%28by%20ref%29))
  (Default|CallSelectionTriggerEvent 4 "/Game/Blueprints/PinkBall.PinkBall_C" 10))

(event OnComponentBeginOverlap(GoldTrigger)
  (params (OverlappedComponent :type Primitive%20Component%20Object%20Reference) (OtherActor :type Actor%20Object%20Reference) (OtherComp :type Primitive%20Component%20Object%20Reference) (OtherBodyIndex :type Integer) (bFromSweep :type Boolean) (SweepResult :type Hit%20Result%20Structure%20%28by%20ref%29))
  (Default|CallSelectionTriggerEvent 2 "/Game/Blueprints/GoldBall.GoldBall_C" 100))

(event OnComponentBeginOverlap(IceTrigger)
  (params (OverlappedComponent :type Primitive%20Component%20Object%20Reference) (OtherActor :type Actor%20Object%20Reference) (OtherComp :type Primitive%20Component%20Object%20Reference) (OtherBodyIndex :type Integer) (bFromSweep :type Boolean) (SweepResult :type Hit%20Result%20Structure%20%28by%20ref%29))
  (Default|CallSelectionTriggerEvent 1 "/Game/Blueprints/IceBall.IceBall_C" 200))

(event OnComponentBeginOverlap(FireTrigger)
  (params (OverlappedComponent :type Primitive%20Component%20Object%20Reference) (OtherActor :type Actor%20Object%20Reference) (OtherComp :type Primitive%20Component%20Object%20Reference) (OtherBodyIndex :type Integer) (bFromSweep :type Boolean) (SweepResult :type Hit%20Result%20Structure%20%28by%20ref%29))
  (Default|CallSelectionTriggerEvent 3 "/Game/Blueprints/FireBall.FireBall_C" 20))

(event OnComponentBeginOverlap(StandardTrigger)
  (params (OverlappedComponent :type Primitive%20Component%20Object%20Reference) (OtherActor :type Actor%20Object%20Reference) (OtherComp :type Primitive%20Component%20Object%20Reference) (OtherBodyIndex :type Integer) (bFromSweep :type Boolean) (SweepResult :type Hit%20Result%20Structure%20%28by%20ref%29))
  (Default|CallSelectionTriggerEvent 0 "/Game/Blueprints/PaperBall.PaperBall_C"))

(event Custom|TriggerSelection
  (params (Index :type Integer) (BallType :type Actor%20Class%20Reference) (Price :type Integer))
  (bind _playermoney (Variables|Default|GetPlayerMoney))
  (if (Utilities|Array|Get(acopy) (Variables|Default|GetPurchased) Index)
    (if (not (== (Variables|Default|GetSelection) Index))
      (bind _returnvalue (Actor|GetActorOfClass "/Game/Blueprints/Paperstack.Paperstack_C"))
      (Default|CallChangeBallEvent _returnvalue BallType)
      (CallFunction|ClearSelection)
      (Rendering|Components|TextRender|SetText (Utilities|Array|Get(acopy) (Variables|Default|GetSelectionTexts) Index) (Utilities|Text|ToText(String) "Selected"))
      (Variables|Default|SetSelection Index))
    (elif (>= _playermoney Price)
      (Default|CallPurchaseEvent (- _playermoney Price))
      (Utilities|Array|SetArrayElem (Variables|Default|GetPurchased) Index true))))

(event EventBeginPlay
  (Variables|Default|SetSelectionTexts (Utilities|Array|MakeArray (Variables|Default|GetStandardText) (Variables|Default|GetIceEffectCost) (Variables|Default|GetgoldPaperCost) (Variables|Default|GetFireEffectCost) (Variables|Default|GetPinkPaperCost)))
  (Variables|Default|SetPurchased (Utilities|Array|MakeArray true false false false false))
  (EventDispatchers|BindEventtoSelectionTriggerEvent (delegate Custom|TriggerSelection)))

(fn ConstructionScript)

(fn ClearSelection
  (for (_array_element _array_index) (Variables|Default|GetSelectionTexts)
    (if (Utilities|Array|Get(acopy) (Variables|Default|GetPurchased) _array_index)
      (Rendering|Components|TextRender|SetText _array_element (Utilities|Text|ToText(String) "")))))