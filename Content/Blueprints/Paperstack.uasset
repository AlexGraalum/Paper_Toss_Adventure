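; Paper stack actor that spawns a throwable-style ball, a paper ball by default, when the VR pawn touches it.
; A ChangeBall event, bound at BeginPlay, sets which ball class spawns.
; On collision overlap it spawns that ball at the stack's transform, scaled down, and plays a crumpling sound.
; A PaperPresent flag blocks further spawns and is not cleared within this Blueprint after play begins.
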(event OnComponentBeginOverlap(PaperStackCollision)
  (params (OverlappedComponent :type Primitive%20Component%20Object%20Reference) (OtherActor :type Actor%20Object%20Reference) (OtherComp :type Primitive%20Component%20Object%20Reference) (OtherBodyIndex :type Integer) (bFromSweep :type Boolean) (SweepResult :type Hit%20Result%20Structure%20%28by%20ref%29))
  ;[1 1 1] On Overlap Construct Paper Ball
  (if (not (Variables|Default|GetPaperPresent))
    (Utilities|Casting|CastToVRPawn OtherActor)
    (bind _returnvalue (Game|SpawnActorfromClass (Variables|Default|GetChosen%20Ball) (Variables|Default|Getcounter_actor_start) "Undefined" 0 0))
    (bind _output_get (Variables|Default|SetCurrentBall _returnvalue))
    (Variables|Default|SetPaperPresent true)
    (Audio|PlaySoundatLocation "/Game/Audio/mixkit-crumpled-paper-2389.mixkit-crumpled-paper-2389" (Transformation|GetActorLocation _output_get) "0, 0, 0" 1.0 1.0 0.0 0 0 0)))

(event Custom|ChangeBall
  (params (NewBall :type Actor%20Class%20Reference))
  (Variables|Default|SetChosen%20Ball NewBall))

(event EventBeginPlay
  (bind _returnvalue (Transformation|GetActorTransform))
  (bind (_location _rotation) (Math|Transform|BreakTransform _returnvalue))
  ;[1 1 1] Set Spawner Safety and Location
  (Variables|Default|SetPaperPresent false)
  (Variables|Default|Setcounter_actor_start (Math|Transform|MakeTransform _location _rotation "0.125000,0.125000,0.125000"))
  (EventDispatchers|BindEventtoChangeBallEvent (delegate Custom|ChangeBall))
  (CallFunction|ChangeBall "/Game/Blueprints/PaperBall.PaperBall_C"))

(fn ConstructionScript)